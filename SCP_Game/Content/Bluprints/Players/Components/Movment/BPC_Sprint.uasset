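; BPC_Sprint is a player component that handles hold-to-sprint movement with a stamina pool.
; On BeginPlay it adds the default input mapping and caches walk and sprint speeds and CharacterMovement from the player character.
; IA_Sprint raises speed and starts a depletion timer if stamina remains; only releasing it restores walk speed.
; Tick re-sets a looping regeneration timer every non-sprinting frame, and that timer is never cleared.
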(event Custom|AddStamina
  (bind _output_get (Variables|Default|SetStamina (Math|Float|Clamp(Float) (+ (Variables|Default|GetStamina) 1.0) 0.0 (Variables|Default|GetMax%20Stamina))))
  (Development|PrintString (Utilities|String|ToString(Float) _output_get)))

(event Custom|RemoveStamina
  ;[0.15 0.15 0.15 0.5] Sprint
  (bind _output_get (Variables|Default|SetStamina (Math|Float|Clamp(Float) (- (Variables|Default|GetStamina) 1.0) 0.0 (Variables|Default|GetMax%20Stamina))))
  (Development|PrintString (Utilities|String|ToString(Float) _output_get)))

(event Input|EnhancedActionEvents|EnhancedInputActionIA_Sprint
  (params (ActionValue :type Boolean) (ElapsedSeconds :type Float%20%28double-precision%29) (TriggeredSeconds :type Float%20%28double-precision%29) (InputAction :type Input%20Action%20Object%20Reference :default "/Game/Bluprints/Inputs/Inputs/IA_Sprint.IA_Sprint"))
  ;[0.15 0.15 0.15 0.5] Sprint
  (:Started
    (if (> (Variables|Default|GetStamina) 0.0)
      (Variables|Default|SetisSprinting? true)
      (Variables|/Script/Engine.CharacterMovementComponent|SetMaxWalkSpeed (Variables|Default|GetCharacter%20Movement) (Variables|Default|GetSprint%20Max%20Movment%20Speed))
      (bind _returnvalue (Utilities|Time|SetTimerbyEvent (delegate Custom|RemoveStamina) (Variables|Default|GetStamina%20Increase%20Time) (> (Variables|Default|GetStamina) 0.0)))
      (Variables|Default|SetDepletion%20Timer _returnvalue)))
  (:Completed
    (Variables|Default|SetisSprinting? false)
    (Variables|/Script/Engine.CharacterMovementComponent|SetMaxWalkSpeed (Variables|Default|GetCharacter%20Movement) (Variables|Default|GetMax%20Walk%20Speed))
    (Utilities|Time|ClearandInvalidateTimerbyHandle (Variables|Default|GetDepletion%20Timer))))

(event EventBeginPlay
  (bind _aspc_deafult (Utilities|Casting|CastToPC_Deafult (Game|GetPlayerController 0)))
  (Input|AddMappingContext (PlayerController|LocalPlayerSubsystems|GetEnhancedInputLocalPlayerSubsystem _aspc_deafult) "/Game/Bluprints/Inputs/IMC_Deafult.IMC_Deafult" 0 "(bIgnoreAllPressedKeysUntilRelease=True,bForceImmediately=False,bNotifyUserSettings=False)")
  (bind _asbp_deafult_player (Utilities|Casting|CastToBP_DeafultPlayer (Game|GetPlayerCharacter 0)))
  (Variables|Default|SetMax%20Walk%20Speed (Variables|/Game/Bluprints/Players/BP_DeafultPlayer.BP_DeafultPlayer_C|GetMaxWalkSpeed _asbp_deafult_player))
  (Variables|Default|SetSprint%20Max%20Movment%20Speed (Variables|/Game/Bluprints/Players/BP_DeafultPlayer.BP_DeafultPlayer_C|GetSprintMaxMovmentSpeed _asbp_deafult_player))
  (bind _asbp_deafult_player_2 (Utilities|Casting|CastToBP_DeafultPlayer (Game|GetPlayerCharacter 0)))
  (Variables|Default|SetCharacter%20Movement (Variables|/Script/Engine.Character|GetCharacterMovement _asbp_deafult_player_2)))

(event EventTick
  (params (DeltaSeconds :type Float%20%28single-precision%29))
  (if (not (Variables|Default|GetisSprinting?))
    (Utilities|Time|SetTimerbyEvent (delegate Custom|AddStamina) (Variables|Default|GetStamina%20Increase%20Time) true)))