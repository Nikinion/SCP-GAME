(event EventBeginPlay
  (bind _returnvalue (UserInterface|CreateWidget "/Game/UI/WigetBluprint/Inventory/WB_Inventory.WB_Inventory_C"))
  (Variables|Default|SetInventoryWidget _returnvalue)
  (Utilities|Array|Resize (Variables|Default|GetItems) 8)
  (Default|LoadInventory (Variables|Default|GetInventoryWidget) self))

(event EventInteraction)

(event Input|KeyboardEvents|I
  (params (Key :type Key%20Structure))
  (bind _inventorywidget (Variables|Default|GetInventoryWidget))
  (:Pressed
    (bind _aspc_deafult (Utilities|Casting|CastToPC_Deafult (Game|GetPlayerController 0)))
    (Variables|/Script/Engine.PlayerController|SetbShowMouseCursor _aspc_deafult true)
    (if (Widget|IsVisible (Variables|Default|GetInventoryWidget))
      (Widget|RemovefromParent _inventorywidget)
      (Variables|/Script/Engine.PlayerController|SetbShowMouseCursor _aspc_deafult false)
      (else
        (UserInterface|Viewport|AddtoViewport _inventorywidget 0)))))

(event Input|KeyboardEvents|E
  (params (Key :type Key%20Structure))
  (bind _returnvalue (Game|GetPlayerCharacter 0))
  (bind _returnvalue_2 (Transformation|GetActorLocation _returnvalue))
  (bind _returnvalue_3 (- _returnvalue_2 "0.000000,20.000000,65.000000"))
  (:Pressed
    (bind _outhit (Collision|SphereTraceByChannel _returnvalue_3 _returnvalue_3 1.2e+02 "TraceTypeQuery1" false 0 "ForDuration"))
    (bind _asbp_deafult_item (Utilities|Casting|CastToBP_DeafultItem (.HitActor (Collision|BreakHitResult _outhit))))
    (for (_array_element _array_index) (Variables|Default|GetItems)
      (Utilities|IsValid _asbp_deafult_item
        (:Is%20Valid
          (if (Math|Boolean|ANDBoolean (Utilities|Enum|Equal(Enum) (.Name (Utilities|Struct|BreakST_Item _array_element)) (.Name (Utilities|Struct|BreakST_Item (Variables|/Game/Bluprints/Inventory/Items/BP_DeafultItem.BP_DeafultItem_C|GetItem _asbp_deafult_item)))) (.Stacble (Utilities|Struct|BreakST_Item (Variables|/Game/Bluprints/Inventory/Items/BP_DeafultItem.BP_DeafultItem_C|GetItem _asbp_deafult_item))) (<= (+ (.Quantity (Utilities|Struct|BreakST_Item _array_element)) (.Quantity (Utilities|Struct|BreakST_Item (Variables|/Game/Bluprints/Inventory/Items/BP_DeafultItem.BP_DeafultItem_C|GetItem _asbp_deafult_item)))) 64))
            (Utilities|Array|SetArrayElem (Variables|Default|GetItems) _array_index (Utilities|Struct|MakeST_Item (.name (Variables|/Game/Bluprints/Inventory/Items/BP_DeafultItem.BP_DeafultItem_C|GetItem _asbp_deafult_item)) (.description (Variables|/Game/Bluprints/Inventory/Items/BP_DeafultItem.BP_DeafultItem_C|GetItem _asbp_deafult_item)) false (.stacble (Variables|/Game/Bluprints/Inventory/Items/BP_DeafultItem.BP_DeafultItem_C|GetItem _asbp_deafult_item)) (+ (.Quantity (Utilities|Struct|BreakST_Item _array_element)) (.Quantity (Utilities|Struct|BreakST_Item (Variables|/Game/Bluprints/Inventory/Items/BP_DeafultItem.BP_DeafultItem_C|GetItem _asbp_deafult_item)))) (.thumbnai (Variables|/Game/Bluprints/Inventory/Items/BP_DeafultItem.BP_DeafultItem_C|GetItem _asbp_deafult_item)) (.mesh (Variables|/Game/Bluprints/Inventory/Items/BP_DeafultItem.BP_DeafultItem_C|GetItem _asbp_deafult_item))))
            (Default|LoadInventory (Variables|Default|GetInventoryWidget) self :!label _label)
            (Actor|DestroyActor _asbp_deafult_item)
            (elif (== (.Quantity (Utilities|Struct|BreakST_Item _array_element)) 0)
              (Utilities|Array|SetArrayElem (Variables|Default|GetItems) _array_index (Variables|/Game/Bluprints/Inventory/Items/BP_DeafultItem.BP_DeafultItem_C|GetItem _asbp_deafult_item))
              (goto _label))))))))